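; Stripped-down player controller variant of the painter game, named for video use, that possesses the first BP_PlayerCharacterBase found on BeginPlay.
; Keys 1-3 activate the matching VideoRefillers entry on BP_PainterGameMode.
; Key O debug-prints each bucket's grabbable component and its owner.
; HUD, pause, win/lose menus, character cycling and customer-list logic are left disconnected, including the binding for the customer-removal handler.
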(event `Key|One`
  (params (Key :type "Key Structure"))
  (:`Pressed`
    (`/Game/InteractiveObjects/Blueprints/Common/BP_InteractiveActorBase.Activate` (`|GetArrayItem` (`/Game/Core/BP_PainterGameMode.VideoRefillers` (cast `/Game/Core/BP_PainterGameMode` (`GameplayStatics.GetGameMode`) :!pure true))))))

(event `Key|Two`
  (params (Key :type "Key Structure"))
  (:`Pressed`
    (`/Game/InteractiveObjects/Blueprints/Common/BP_InteractiveActorBase.Activate` (`|GetArrayItem` (`/Game/Core/BP_PainterGameMode.VideoRefillers` (cast `/Game/Core/BP_PainterGameMode` (`GameplayStatics.GetGameMode`) :!pure true)) 1))))

(event `Key|Three`
  (params (Key :type "Key Structure"))
  (:`Pressed`
    (`/Game/InteractiveObjects/Blueprints/Common/BP_InteractiveActorBase.Activate` (`|GetArrayItem` (`/Game/Core/BP_PainterGameMode.VideoRefillers` (cast `/Game/Core/BP_PainterGameMode` (`GameplayStatics.GetGameMode`) :!pure true)) 2))))

(event `Key|O`
  (params (Key :type "Key Structure"))
  (:`Pressed`
    (bind _outactors (`GameplayStatics.GetAllActorsOfClass` "/Game/InteractiveObjects/Blueprints/BP_Bucket.BP_Bucket_C"))
    (for _array_element _outactors
      (bind _bpc_grabbablecomponent (`/Game/InteractiveObjects/Blueprints/BP_Bucket.BPC_GrabbableComponent` _array_element))
      (`KismetSystemLibrary.PrintString` (`KismetSystemLibrary.GetDisplayName` _bpc_grabbablecomponent))
      (`KismetSystemLibrary.PrintString` (`KismetSystemLibrary.GetDisplayName` (`ActorComponent.GetOwner` _bpc_grabbablecomponent))))))

(event `ControllerLoseEvent`)

(event `ControllerWonEvent`)

(event `InputAction|MyPause`
  (params (Key :type "Key Structure")))

(event `self.ReceiveBeginPlay`
  (bind _outactors (`GameplayStatics.GetAllActorsOfClass` "/Game/Core/PlayerCharacter/BP_PlayerCharacterBase.BP_PlayerCharacterBase_C"))
  (bind _output_get (set `self.AvailablePlayerCharacters` _outactors))
  (`self.Possess` (`|GetArrayItem` _output_get)))

(event `RemoveCustomerEventD_Event_0`
  (`KismetArrayLibrary.Array_Remove` (`self.ControllerCustomerList`) (`/Game/Core/BP_PainterGameMode.IndexToRemoveCustomer` (cast `/Game/Core/BP_PainterGameMode` (`GameplayStatics.GetGameMode`) :!pure true))))

(event `InputAction|PossesAnotherCharacter`
  (params (Key :type "Key Structure")))

(event `AddCustomer`
  (params (Customer :type "/Game/UI/S_CustomerStructure Structure")))

(fn `UserConstructionScript`)