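; Base player character Blueprint with world-axis movement, a forward dash launch and an interact action.
; Interact runs a vertical sphere trace at the grab offset ahead of the character to find BP_InteractiveActorBase actors, ignoring the held object.
; The target's interact type selects either a click message or grab/release through BPC_GrabbableComponent, holding one object at a time.
; Interacting without a valid target also releases the held object.
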(event `InputAxis|MoveForward`
  (params (AxisValue :type "Float (single-precision)"))
  (`self.AddMovementInput` (1.0 0.0 0.0) AxisValue))

(event `InputAxis|MoveRight`
  (params (AxisValue :type "Float (single-precision)"))
  (`self.AddMovementInput` (0.0 1.0 0.0) AxisValue))

(event `InputAction|Dash`
  (params (Key :type "Key Structure"))
  (:`Pressed`
    (`self.LaunchCharacter` (* (`self.GetActorForwardVector`) (`self.DashIntensity`)))))

(event `InputAction|Interact`
  (params (Key :type "Key Structure"))
  (bind _returnvalue (* (`self.GetActorUpVector`) (`self.InteractUpHalfDistance`)))
  (bind _returnvalue_2 (+ (`self.K2_GetActorLocation`) (* (`self.GetActorForwardVector`) (.x (`SceneComponent.RelativeLocation` (`self.GrabLocationSceneComponent`))))))
  (:`Pressed`
    (bind _outhit (`KismetSystemLibrary.SphereTraceSingleForObjects` (+ _returnvalue_2 (/ _returnvalue 2.0)) (+ _returnvalue_2 (* _returnvalue -1.0)) 30.0 (`|MakeArray` "ObjectTypeQuery2" :!type "EObjectTypeQuery Enum") false (`|MakeArray` (`self.GrabbedObj`) :!type "Actor Object Reference") "None" true (struct :`R` 1.0 :`A` 1.0) (struct :`G` 1.0 :`A` 1.0) 0.25))
    (bind (_bblockinghit _binitialoverlap _time _distance _location _impactpoint _normal _impactnormal _physmat _hitactor) (`GameplayStatics.BreakHitResult` _outhit))
    (bind _asbp_interactive_actor_base (cast `/Game/InteractiveObjects/Blueprints/Common/BP_InteractiveActorBase` _hitactor)
      (:`then`
        (bind _output_get (set `self.InteractiveActorBaseRef` _asbp_interactive_actor_base))
        (switch `/Game/InteractiveObjects/Blueprints/Common/EInteractiveType` (`/Game/InteractiveObjects/Blueprints/Common/BP_InteractiveActorBase.EInteractType` _output_get)
          (:`NewEnumerator0`
            (message `/Game/Core/BPI_Interact.PainterInteract` (`self.InteractiveActorBaseRef`) self))
          (:`NewEnumerator2`
            (if (== (`self.GrabbedObj`) null)
              (bind _returnvalue_3 (`self.GetComponentByClass` _asbp_interactive_actor_base "/Game/InteractiveObjects/Blueprints/Common/BPC_GrabbableComponent.BPC_GrabbableComponent_C"))
              (if (`/Game/InteractiveObjects/Blueprints/Common/BPC_GrabbableComponent.bCanBeGrabbed` _returnvalue_3)
                (set `self.GrabbedObj` (`self.InteractiveActorBaseRef`))
                (`/Game/InteractiveObjects/Blueprints/Common/BPC_GrabbableComponent.GetGrabbed` _returnvalue_3 self)
                (else
                  (`KismetSystemLibrary.PrintString` "Actor Can not Be Grabbed ATM" true true (struct :`R` 1.0 :`G` 0.432906 :`A` 1.0))))
              (else
                (`/Game/InteractiveObjects/Blueprints/Common/BPC_GrabbableComponent.GetReleased` (`self.GetComponentByClass` (`self.GrabbedObj`) "/Game/InteractiveObjects/Blueprints/Common/BPC_GrabbableComponent.BPC_GrabbableComponent_C") _impactpoint :!label _label)
                (set `self.GrabbedObj` null))))))
      (:`CastFailed`
        (if (!= (`self.GrabbedObj`) null)
          (goto _label))))))

(fn `UserConstructionScript`)