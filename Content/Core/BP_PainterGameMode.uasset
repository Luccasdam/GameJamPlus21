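; Game mode for a paint-mixing level that runs the countdown, customer orders and win or lose check.
; Looping timers tick the clock and add random RGB colour orders, capped at four active and a level maximum, broadcasting changes through dispatchers.
; Time running out, or optionally reaching the submission target, pauses the game and reports the result to BP_PainterController.
; Buckets respawn at indexed locations after a delay, with two pending-index slots.
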(event `RespawnBucket`
  (params (SpawnIndex :type Integer))
  (bind _bucketindextospawn (`self.BucketIndexToSpawn`))
  (bind _secondbucketindextospawn (`self.SecondBucketIndexToSpawn`))
  ;[1 1 1] ReSpawn Bucket
  (if (not (`self.bWaitingToSpawn`))
    (set `self.bWaitingToSpawn` true)
    (set `self.BucketIndexToSpawn` SpawnIndex)
    (`KismetSystemLibrary.Delay` 3.0)
    (set `self.bWaitingToSpawn` false)
    (`|SpawnActorFromClass` "/Game/InteractiveObjects/Blueprints/BP_Bucket.BP_Bucket_C" (`KismetMathLibrary.MakeTransform` (`|GetArrayItem` (`self.BucketRespawLocation`) _bucketindextospawn)) "Undefined" "OverrideRootScale" null _bucketindextospawn null)
    (else
      (set `self.SecondBucketIndexToSpawn` SpawnIndex)
      (`KismetSystemLibrary.Delay` 3.0)
      (`|SpawnActorFromClass` "/Game/InteractiveObjects/Blueprints/BP_Bucket.BP_Bucket_C" (`KismetMathLibrary.MakeTransform` (`|GetArrayItem` (`self.BucketRespawLocation`) _secondbucketindextospawn)) "Undefined" "OverrideRootScale" null _secondbucketindextospawn null))))

(event `UpdateCustomerSubmissions`
  (params (bIncrementSubmissions :type Boolean))
  (bind _correctcustomerssubmissions (`self.CorrectCustomersSubmissions`))
  (if bIncrementSubmissions
    (`/Engine/EditorBlueprintResources/StandardMacros.IncrementInt` _correctcustomerssubmissions
      (:`  `
        _)))
  (`self.CustomersRemaining`)
  (if (and (== (- (`self.WinConditionMinCustomersSubmissions`) _correctcustomerssubmissions) 0) (`self.bWinByCustomerCount`))
    (`self.CheckWinCondition`)))

(event `self.ReceiveBeginPlay`
  ;[0.2573 1 0.1697] BeginPLlay
  (`KismetSystemLibrary.K2_SetTimerDelegate` (delegate `TimeCountdown`) 1.0 true)
  (bind _returnvalue (`KismetSystemLibrary.K2_SetTimerDelegate` (delegate `NewCustomerOrder`) (`KismetMathLibrary.RandomFloatInRange` (`self.MinCustomerTimer`) (`self.MaxCustomerTimer`)) true))
  (set `self.CustomerAddTimerHandle` _returnvalue))

(event `TimeCountdown`
  ;[1 1 1] TimeCountdown
  (bind _result (`/Engine/EditorBlueprintResources/StandardMacros.DecrementFloat` (`self.LevelTime`))
    (:`  `
      (if (!= _result 0.0)
        (`self.TimeCountdown_EventD`)
        (else
          (`self.CheckWinCondition`)
          (`GameplayStatics.SetGamePaused` true))))))

(event `NewCustomerOrder`
  (bind _customerindex (`self.CustomerIndex`))
  (bind _maxtintintensity (`self.MaxTintIntensity`))
  (bind _returnvalue (`KismetMathLibrary.Conv_IntToDouble` (`KismetMathLibrary.RandomIntegerInRange` 0 _maxtintintensity)))
  (bind _returnvalue_2 (`KismetMathLibrary.Conv_IntToDouble` (`KismetMathLibrary.RandomIntegerInRange` 0 _maxtintintensity)))
  (bind _returnvalue_3 (`KismetMathLibrary.Conv_IntToDouble` (`KismetMathLibrary.RandomIntegerInRange` 0 _maxtintintensity)))
  (bind _returnvalue_4 (+ _returnvalue_2 _returnvalue_3 _returnvalue))
  (if (< (`KismetArrayLibrary.Array_Length` (`self.ActiveCustomers`)) 4) :!label _label
    (if (and (> _returnvalue_4 0.0) (>= (`self.MaxCustomerDesiredColorIntensity`) _returnvalue_4))
      (if (not (>= _customerindex (- (`self.MaxCustomers`) 1)))
        (bind _result (`/Engine/EditorBlueprintResources/StandardMacros.IncrementInt` _customerindex)
          (:`  `
            (bind _s_customerstructure (make `/Game/UI/S_CustomerStructure` _result (+ (`KismetMathLibrary.MakeVector` (* 0.2 _returnvalue_2) (* 0.2 _returnvalue_3) (* 0.2 _returnvalue)) (select `int` (`KismetMathLibrary.RandomIntegerInRange` 0 2) :`0` (`KismetMathLibrary.MakeVector` 0.2) :`1` (`KismetMathLibrary.MakeVector` 0.0 0.2) :`2` (`KismetMathLibrary.MakeVector` 0.0 0.0 0.2)))))
            (`KismetArrayLibrary.Array_Add` (`self.CustomerStructure`) _s_customerstructure)
            (`KismetArrayLibrary.Array_Add` (`self.ActiveCustomers`) _s_customerstructure)
            (`self.NewCustomerEventD`)))
        (else
          (`KismetSystemLibrary.K2_ClearAndInvalidateTimerHandle` (`self.CustomerAddTimerHandle`))))
      (else
        (`KismetSystemLibrary.Delay` 0.2)
        (goto _label)))))

(event `RemoveSatisfiedCustomer`
  (params (IndexToRemove :type Integer))
  ;[1 1 1] Remove Customers
  (`KismetArrayLibrary.Array_Remove` (`self.ActiveCustomers`) IndexToRemove)
  (set `self.IndexToRemoveCustomer` IndexToRemove)
  (`self.RemoveCustomerEventD`))

(event `CheckWinCondition`
  (bind _asbp_painter_controller (cast `/Game/Core/BP_PainterController` (`GameplayStatics.GetPlayerController` 0) :!pure true))
  ;[1 1 1] WinCondition
  (if (>= (`self.CorrectCustomersSubmissions`) (`self.WinConditionMinCustomersSubmissions`))
    (`/Game/Core/BP_PainterController.ControllerWonEvent` _asbp_painter_controller)
    (else
      (`/Game/Core/BP_PainterController.ControllerLoseEvent` _asbp_painter_controller)))
  (`GameplayStatics.SetGamePaused` true))

(fn `UserConstructionScript`)