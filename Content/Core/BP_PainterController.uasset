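; BP_PainterController is the player controller that lets the player cycle possession through the level's BP_PlayerCharacterBase characters on input.
; On BeginPlay it gathers those characters, possesses the first, stores the BP_PainterCamera and shows the HUD.
; It keeps a customer list, filled through AddCustomer and trimmed by a BP_PainterGameMode dispatcher using the game mode's index.
; Pause, win and lose events show their menus and the cursor.
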(event `ControllerLoseEvent`
  (set `self.bShowMouseCursor` true)
  (`GameplayStatics.SpawnSound2D` "/Game/Audio/GameOver.GameOver" 1.0 1.0 0.0 null)
  (bind _returnvalue (`|CreateWidget` "/Game/UI/Menu/WBP_LoseMenu.WBP_LoseMenu_C" self))
  (`UserWidget.AddToViewport` _returnvalue 0))

(event `ControllerWonEvent`
  (set `self.bShowMouseCursor` true)
  (`GameplayStatics.SpawnSound2D` "/Game/Audio/CorrectDelivery.CorrectDelivery" 1.0 1.0 0.0 null)
  (bind _returnvalue (`|CreateWidget` "/Game/UI/Menu/WBP_WinMenu.WBP_WinMenu_C" self))
  (`UserWidget.AddToViewport` _returnvalue 0))

(event `InputAction|MyPause`
  (params (Key :type "Key Structure"))
  (:`Pressed`
    (bind _returnvalue (`|CreateWidget` "/Game/UI/Menu/WBP_PauseMenu.WBP_PauseMenu_C" self))
    (`UserWidget.AddToViewport` _returnvalue 0)
    (set `self.bShowMouseCursor` true)
    (`GameplayStatics.SetGamePaused` true)))

(event `self.ReceiveBeginPlay`
  (bind _outactors (`GameplayStatics.GetAllActorsOfClass` "/Game/Core/PlayerCharacter/BP_PlayerCharacterBase.BP_PlayerCharacterBase_C"))
  (bind _output_get (set `self.AvailablePlayerCharacters` _outactors))
  (`self.Possess` (`|GetArrayItem` _output_get))
  (bind _returnvalue (`GameplayStatics.GetActorOfClass` "/Game/Core/BP_PainterCamera.BP_PainterCamera_C"))
  (set `self.LevelCamera` _returnvalue)
  (bind _returnvalue_2 (`|CreateWidget` "/Game/UI/WBP_UI.WBP_UI_C" self))
  (`UserWidget.AddToViewport` _returnvalue_2 0)
  (set `self.PlayerUI` _returnvalue_2)
  (add `/Game/Core/BP_PainterGameMode.RemoveCustomerEventD` (cast `/Game/Core/BP_PainterGameMode` (`GameplayStatics.GetGameMode`) :!pure true) (delegate `RemoveCustomerEventD_Event_0`))
  (set `self.bShowMouseCursor` false))

(event `RemoveCustomerEventD_Event_0`
  (`KismetArrayLibrary.Array_Remove` (`self.ControllerCustomerList`) (`/Game/Core/BP_PainterGameMode.IndexToRemoveCustomer` (cast `/Game/Core/BP_PainterGameMode` (`GameplayStatics.GetGameMode`) :!pure true))))

(event `InputAction|PossesAnotherCharacter`
  (params (Key :type "Key Structure"))
  (:`Pressed`
    (if (!= (`self.CurrentCharacterIndex`) (`KismetArrayLibrary.Array_LastIndex` (`self.AvailablePlayerCharacters`)))
      (`/Engine/EditorBlueprintResources/StandardMacros.IncrementInt` (`self.CurrentCharacterIndex`)
        (:`  `
          _))
      (else
        (set `self.CurrentCharacterIndex` 0)))
    (`self.Possess` (`|GetArrayItem` (`self.AvailablePlayerCharacters`) (`self.CurrentCharacterIndex`)))))

(event `AddCustomer`
  (params (Customer :type "/Game/UI/S_CustomerStructure Structure"))
  (`KismetArrayLibrary.Array_Add` (`self.ControllerCustomerList`) Customer))

(fn `UserConstructionScript`)