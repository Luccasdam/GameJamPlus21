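; BP_PlayerCharacterBase is the base player character, handling world-axis movement, a forward dash and interaction with objects.
; Movement inputs feed AddMovementInput, while Dash launches the character along its forward vector scaled by DashIntensity.
; Interact runs a debug-drawn vertical sphere trace at the grab point's forward offset, then sends PainterInteractMessage to the hit actor with the character, grabbed object and inverted grab state.
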(event `InputAxis|MoveForward`
  (params (AxisValue :type "Float (single-precision)"))
  (`self.AddMovementInput` (1.0 0.0 0.0) AxisValue))

(event `InputAxis|MoveRight`
  (params (AxisValue :type "Float (single-precision)"))
  (`self.AddMovementInput` (0.0 1.0 0.0) AxisValue))

(event `InputAction|Dash`
  (params (Key :type "Key Structure"))
  (:`Pressed`
    (`self.LaunchCharacter` (* (`self.GetActorForwardVector`) (`self.DashIntensity`)))))

(event `InputAction|Interact`
  (params (Key :type "Key Structure"))
  (bind _returnvalue (* (`self.GetActorUpVector`) (`self.InteractUpHalfDistance`)))
  (bind _returnvalue_2 (+ (`self.K2_GetActorLocation`) (* (`self.GetActorForwardVector`) (.x (`SceneComponent.RelativeLocation` (`self.GrabLocationSceneComponent`))))))
  (:`Pressed`
    (bind _outhit (`KismetSystemLibrary.SphereTraceSingleForObjects` :`Start` (+ _returnvalue_2 _returnvalue) :`End` (+ _returnvalue_2 (* _returnvalue -1.0)) :`Radius` 30.0 :`ObjectTypes` (`|MakeArray` "ObjectTypeQuery2" :!type "EObjectTypeQuery Enum") :`DrawDebugType` "Persistent" :`DrawTime` 0.25))
    (message `/Game/Core/BPI_Interact.PainterInteract` (`.HitActor` (`GameplayStatics.BreakHitResult` _outhit)) self (`self.GrabbedObj`) (not (`self.bGrabbing`)))))

(fn `UserConstructionScript`)