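; BP_Refiller is an activatable refiller object that tracks an interactive actor inside its box and animates its mesh.
; Box overlaps store any BP_InteractiveActorBase as ActorToRefill and clear it when that actor leaves.
; Activate prints an initialization message, then plays the Refill timeline, which drives the mesh's relative height down from an offset as the track rises.
; The stored actor is not yet refilled or otherwise used on activation.
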(event `self.Box.OnComponentBeginOverlap`
  (params (OverlappedComponent :type "PrimitiveComponent Object Reference") (OtherActor :type "Actor Object Reference") (OtherComp :type "PrimitiveComponent Object Reference") (OtherBodyIndex :type Integer) (bFromSweep :type Boolean) (SweepResult :type "HitResult Structure (by ref)"))
  (bind _asbp_interactive_actor_base (cast `/Game/InteractiveObjects/BP_InteractiveActorBase` OtherActor))
  (set `self.ActorToRefill` _asbp_interactive_actor_base))

(event `self.Box.OnComponentEndOverlap`
  (params (OverlappedComponent :type "PrimitiveComponent Object Reference") (OtherActor :type "Actor Object Reference") (OtherComp :type "PrimitiveComponent Object Reference") (OtherBodyIndex :type Integer))
  (bind _actortorefill (`self.ActorToRefill`))
  (if (and (== OtherActor _actortorefill) (`KismetSystemLibrary.IsValid` _actortorefill))
    (set `self.ActorToRefill` null)))

(event `self.Activate`
  (`KismetSystemLibrary.PrintText` (`|FormatText` "{NAME} Initialized" self))
  (bind (_direction _newtrack_0) (`Timeline|Refill` :!via `PlayFromStart`)
    (:`Update`
      (`SceneComponent.K2_SetRelativeLocation` (`self.StaticMesh`) (`KismetMathLibrary.MakeVector` 0.0 0.0 (+ (* _newtrack_0 -100.0) 200.0)) false false))))

(fn `UserConstructionScript`)