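; BP_Delivery is the interactive drop-off point where paint buckets are matched to waiting customers' color orders.
; It registers itself as owner of a child BP_PlaceableTrigger and binds the GameMode's new-customer event, which only logs.
; Releasing a bucket compares its color, within a tolerance, against the controller's customer list; the first match removes that customer, destroys the bucket and reports a successful submission.
; Number keys print customers' requested colors for debugging.
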(event `self.ReceiveBeginPlay`
  (bind _returnvalue (`GameplayStatics.GetPlayerController` 0))
  (`parent.ReceiveBeginPlay`)
  (bind _asbp_placeable_trigger (cast `/Game/InteractiveObjects/Blueprints/Common/BP_PlaceableTrigger` (`ChildActorComponent.ChildActor` (`self.ChildActor1`))))
  (set `/Game/InteractiveObjects/Blueprints/Common/BP_PlaceableTrigger.MyOwner` self _asbp_placeable_trigger)
  (cast `/Game/Core/BP_PainterGameMode` (`GameplayStatics.GetGameMode`))
  (add `/Game/Core/BP_PainterGameMode.NewCustomerEventD` (`self.PainterGameModeRef`) (delegate `NewCustomerEventD_Event_0`))
  (`self.EnableInput` _returnvalue)
  (bind _asbp_painter_controller (cast `/Game/Core/BP_PainterController` _returnvalue))
  (set `self.BP_PainterControllerAgain` _asbp_painter_controller))

(event `NewCustomerEventD_Event_0`
  (`KismetSystemLibrary.PrintString` "Delivery Delegate Assign OnGameMode NewCustomerEvent"))

(event `/Game/Core/BPI_Interact.Release Interact`
  (params (ReleasedInteractiveActor :type "/Game/InteractiveObjects/Blueprints/Common/BP_InteractiveActorBase Object Reference"))
  (bind _asbp_bucket (cast `/Game/InteractiveObjects/Blueprints/BP_Bucket` ReleasedInteractiveActor))
  (bind _asbp_painter_controller (cast `/Game/Core/BP_PainterController` (`GameplayStatics.GetPlayerController` 0)))
  (if (`KismetArrayLibrary.Array_IsValidIndex` (`/Game/Core/BP_PainterGameMode.CustomerStructure` (`self.PainterGameModeRef`)))
    (bind _controllercustomerlist (`/Game/Core/BP_PainterController.ControllerCustomerList` _asbp_painter_controller))
    (for (_array_element _array_index) _controllercustomerlist
      (bind _output_get (set `self.ColorDebug` (`.CustumerColorInPercent_10_C7B6C8DC46ED328E696026B443175EA9` (break `/Game/UI/S_CustomerStructure` _array_element))))
      (if (== _output_get (`/Game/InteractiveObjects/Blueprints/BP_Bucket.BucketColorIntensity` _asbp_bucket) :`ErrorTolerance` 0.05)
        (`KismetSystemLibrary.PrintString` "You got a satisfied Client" true true (struct :`G` 0.411458 :`B` 0.102865 :`A` 1.0))
        (`/Game/Core/BP_PainterGameMode.RemoveSatisfiedCustomer` (`self.PainterGameModeRef`) _array_index)
        (`/Game/InteractiveObjects/Blueprints/BP_Bucket.MyBucketDestroy` _asbp_bucket)
        (`/Game/Core/BP_PainterGameMode.UpdateCustomerSubmissions` (cast `/Game/Core/BP_PainterGameMode` (`GameplayStatics.GetGameMode`) :!pure true) true)
        (break)
        (elif (== (`KismetArrayLibrary.Array_LastIndex` _controllercustomerlist) _array_index)
          (`KismetSystemLibrary.PrintString` "No customer satisfacted"))))))

(event `Key|One`
  (params (Key :type "Key Structure"))
  (:`Pressed`
    (set `self.DebugIndex` 0)
    (`KismetSystemLibrary.PrintString` (`KismetStringLibrary.Conv_VectorToString` (`.CustumerColorInPercent_10_C7B6C8DC46ED328E696026B443175EA9` (break `/Game/UI/S_CustomerStructure` (`|GetArrayItem` (`/Game/Core/BP_PainterController.ControllerCustomerList` (`self.BP_PainterControllerAgain`)) (`self.DebugIndex`))))) true true (struct :`R` 0.536329 :`B` 1.0 :`A` 1.0) :!label _label)))

(event `Key|Two`
  (params (Key :type "Key Structure"))
  (:`Pressed`
    (set `self.DebugIndex` 1)
    (goto _label)))

(event `Key|Three`
  (params (Key :type "Key Structure"))
  (:`Pressed`
    (set `self.DebugIndex` 2)
    (goto _label)))

(event `Key|Four`
  (params (Key :type "Key Structure"))
  (:`Pressed`
    (set `self.DebugIndex` 3)
    (goto _label)))

(fn `UserConstructionScript`
  (`parent.UserConstructionScript`))