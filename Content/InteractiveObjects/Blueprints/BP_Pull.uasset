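; BP_Pull is an interactive button that activates a linked ActorToActivate when the painter interacts with it.
; The construction script creates a dynamic material for the button light, tinted by the selected EInteractColor.
; PainterInteract calls Activate on the target, plays a 2D sound and runs a timeline that drives the light's emissive intensity.
; CanActivate blocks repeat presses until that animation finishes.
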(event `/Game/Core/BPI_Interact.PainterInteract`
  (params (InstigatorPlayerChar :type "/Game/Core/PlayerCharacter/BP_PlayerCharacterBase Object Reference"))
  (bind _actortoactivate (`self.ActorToActivate`))
  (`/Engine/EditorBlueprintResources/StandardMacros.IsValid` _actortoactivate
    (:`Is Valid`
      (if (`self.bCanActivate`)
        (`self.Activate` _actortoactivate)
        (`GameplayStatics.SpawnSound2D` "/Game/Audio/LataNaMesa.LataNaMesa" 1.0 1.0 0.0 null)
        (set `self.bCanActivate` false)
        (bind (_direction _alpha) (`Timeline|ButtonAnimation` :!via `PlayFromStart`)
          (:`Update`
            (`MaterialInstanceDynamic.SetScalarParameterValue` (`self.Button light material`) "EmissiveIntensity" (* _alpha 5.0)) ; Change a scalar value in the button material that turns it green
          )
          (:`Finished`
            (set `self.bCanActivate` true)))))))

(fn `UserConstructionScript`
  (bind (_red _green _blue _cyan _mangeta _yellow) (break `/Game/InteractiveObjects/Blueprints/Common/SInteractColors` (`self.SInteractColor`)))
  (bind _returnvalue (`PrimitiveComponent.CreateDynamicMaterialInstance` (`self.StaticMesh`) 2 "/Game/Materials/RefillerColor/MI_RefillerColorNeutral.MI_RefillerColorNeutral" "None"))
  (bind _output_get (set `self.Button Light Material` _returnvalue))
  (`MaterialInstanceDynamic.SetVectorParameterValue` _output_get "Color" (`KismetMathLibrary.MakeColor` (.x (select `/Game/InteractiveObjects/Blueprints/Common/EInteractColors` (`self.EInteractColor`) :`NewEnumerator0` _red :`NewEnumerator1` _green :`NewEnumerator2` _blue :`NewEnumerator3` _cyan :`NewEnumerator4` _mangeta :`NewEnumerator5` _yellow)) (.y (select `/Game/InteractiveObjects/Blueprints/Common/EInteractColors` (`self.EInteractColor`) :`NewEnumerator0` _red :`NewEnumerator1` _green :`NewEnumerator2` _blue :`NewEnumerator3` _cyan :`NewEnumerator4` _mangeta :`NewEnumerator5` _yellow)) (.z (select `/Game/InteractiveObjects/Blueprints/Common/EInteractColors` (`self.EInteractColor`) :`NewEnumerator0` _red :`NewEnumerator1` _green :`NewEnumerator2` _blue :`NewEnumerator3` _cyan :`NewEnumerator4` _mangeta :`NewEnumerator5` _yellow)))))