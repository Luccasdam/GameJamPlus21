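; BP_Refiller is an interactive station that refills an interactive actor with its configured RefillColor.
; Its box overlap tracks the latest interactive actor as the target and clears it on exit.
; Activate plays a timeline that moves the mesh vertically, with an event track calling RefillActor on that target.
; The construction script creates dynamic billboard materials showing each RGB component of RefillColor as bar intensity.
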(event `self.ReceiveBeginPlay`)

(event `self.Box.OnComponentBeginOverlap`
  (params (OverlappedComponent :type "PrimitiveComponent Object Reference") (OtherActor :type "Actor Object Reference") (OtherComp :type "PrimitiveComponent Object Reference") (OtherBodyIndex :type Integer) (bFromSweep :type Boolean) (SweepResult :type "HitResult Structure (by ref)"))
  (bind _asbp_interactive_actor_base (cast `/Game/InteractiveObjects/Blueprints/Common/BP_InteractiveActorBase` OtherActor))
  (bind _output_get (set `self.ActorToRefill` _asbp_interactive_actor_base))
  (`KismetSystemLibrary.PrintString` (`KismetSystemLibrary.GetDisplayName` _output_get)))

(event `self.Box.OnComponentEndOverlap`
  (params (OverlappedComponent :type "PrimitiveComponent Object Reference") (OtherActor :type "Actor Object Reference") (OtherComp :type "PrimitiveComponent Object Reference") (OtherBodyIndex :type Integer))
  (bind _actortorefill (`self.ActorToRefill`))
  (if (and (== OtherActor _actortorefill) (`KismetSystemLibrary.IsValid` _actortorefill))
    (bind _output_get (set `self.ActorToRefill` null))
    (`KismetSystemLibrary.PrintString` (`KismetSystemLibrary.GetDisplayName` _output_get))))

(event `self.Activate`
  (bind _actortorefill (`self.ActorToRefill`))
  (`KismetSystemLibrary.PrintText` (`|FormatText` "{NAME} Initialized" self))
  (bind (_direction _newtrack_0) (`Timeline|Refill` :!via `PlayFromStart`)
    (:`Update`
      (`SceneComponent.K2_SetRelativeLocation` (`self.StaticMesh`) (`KismetMathLibrary.MakeVector` 0.0 0.0 (+ (* _newtrack_0 -100.0) 200.0)) false false))
    (:`RefillTargetActor`
      (`/Engine/EditorBlueprintResources/StandardMacros.IsValid` _actortorefill
        (:`Is Valid`
          (`self.RefillActor` _actortorefill (`self.RefillColor`))
          (`KismetSystemLibrary.PrintString` "Hello"))))))

(fn `UserConstructionScript`
  (bind _x (.x (`self.RefillColor`)))
  (`|ExecutionSequence`
    (:`then_0`
      (bind _returnvalue (`PrimitiveComponent.CreateDynamicMaterialInstance` (`self.MaterialBillboard_Red`) 0 "/Game/Materials/ProgressBar/MI_VerticalRedBar.MI_VerticalRedBar" "RedBar"))
      (`MaterialInstanceDynamic.SetScalarParameterValue` _returnvalue "ColorIntensity" _x)
      (bind _returnvalue_2 (`PrimitiveComponent.CreateDynamicMaterialInstance` (`self.MaterialBillboard_Red1`) 0 "/Game/Materials/ProgressBar/MI_RedBar.MI_RedBar" "RedBar"))
      (`MaterialInstanceDynamic.SetScalarParameterValue` _returnvalue_2 "ColorIntensity" _x))
    (:`then_1`
      (bind _returnvalue_3 (`PrimitiveComponent.CreateDynamicMaterialInstance` (`self.MaterialBillboard_Green`) 0 "/Game/Materials/ProgressBar/MI_VerticalGreenBar.MI_VerticalGreenBar" "GreenBar"))
      (`MaterialInstanceDynamic.SetScalarParameterValue` _returnvalue_3 "ColorIntensity" (.y (`self.RefillColor`))))
    (:`then_2`
      (bind _returnvalue_4 (`PrimitiveComponent.CreateDynamicMaterialInstance` (`self.MaterialBillboard_Blue`) 0 "/Game/Materials/ProgressBar/MI_VerticalBlueBar.MI_VerticalBlueBar" "BlueBar"))
      (`MaterialInstanceDynamic.SetScalarParameterValue` _returnvalue_4 "ColorIntensity" (.z (`self.RefillColor`))))))