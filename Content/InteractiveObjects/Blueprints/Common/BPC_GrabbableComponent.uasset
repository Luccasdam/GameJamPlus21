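; Actor component that lets a bucket owner, cast to BP_InteractiveActorBase, be grabbed and released by a player.
; Grabbing attaches it to the player's grab scene component and disables further grabs.
; Release detaches it, then either teleports it to the release point or snaps its XY to the last registered placement actor, notifying that actor through BPI_Interact.
; Player-collision ignore logic is present but unconnected.
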(event `self.ReceiveBeginPlay`
  (bind _asbp_interactive_actor_base (cast `/Game/InteractiveObjects/Blueprints/Common/BP_InteractiveActorBase` (`self.MyOwnerWhoisABucket`)))
  (set `self.OwnerInteractiveBaseRef` _asbp_interactive_actor_base)
  (set `self.bIsThereAPlaceablePlace` false)
  (`KismetArrayLibrary.Array_Clear` (`self.ActorsToBePlaced`))
  (`KismetSystemLibrary.PrintString` (`KismetSystemLibrary.GetObjectName` (`self.GetOwner`)) true true (struct :`R` 0.625 :`G` 0.084689 :`A` 1.0)))

(event `GetGrabbed`
  (params (InstigatorPlayerBase :type "/Game/Core/PlayerCharacter/BP_PlayerCharacterBase Object Reference"))
  (set `self.InstigatorPlayerBase` InstigatorPlayerBase)
  (`Actor.K2_AttachToComponent` (`self.MyOwnerWhoisABucket`) (`/Game/Core/PlayerCharacter/BP_PlayerCharacterBase.GrabLocationSceneComponent` InstigatorPlayerBase) "None" "SnapToTarget" "KeepWorld" "KeepWorld" true)
  (set `self.bCanBeGrabbed` false))

(event `GetReleased`
  (params (ReleaseLocation :type "Vector Structure"))
  (bind _actorstobeplaced (`self.ActorsToBePlaced`))
  (bind _output (`|GetArrayItem` _actorstobeplaced (`KismetArrayLibrary.Array_LastIndex` _actorstobeplaced)))
  (`Actor.K2_DetachFromActor` (`self.MyOwnerWhoisABucket`) "KeepWorld" "KeepWorld" "KeepWorld")
  (if (`self.bIsThereAPlaceablePlace`)
    (if (`KismetArrayLibrary.Array_IsValidIndex` _actorstobeplaced)
      (`Actor.K2_SetActorLocation` (`self.MyOwnerWhoisABucket`) (`KismetMathLibrary.MakeVector` (.x (`Actor.K2_GetActorLocation` _output)) (.y (`Actor.K2_GetActorLocation` _output)) (.z ReleaseLocation)) false true)
      (if (`KismetSystemLibrary.DoesImplementInterface` _output "/Game/Core/BPI_Interact.BPI_Interact_C")
        (`KismetSystemLibrary.PrintString` (`KismetSystemLibrary.GetDisplayName` _output))
        (message `/Game/Core/BPI_Interact.Release Interact` _output (`self.OwnerInteractiveBaseRef`) (`self.MyOwnerWhoisABucket`)))
      (set `self.bCanBeGrabbed` true :!label _label))
    (else
      (`Actor.K2_SetActorLocation` (`self.MyOwnerWhoisABucket`) ReleaseLocation false true)
      (goto _label))))