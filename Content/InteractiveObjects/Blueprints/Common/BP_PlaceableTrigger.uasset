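; BP_PlaceableTrigger is a trigger volume that marks a place where grabbable objects can be released.
; On overlap, it gives the other actor's BPC_GrabbableComponent its MyOwner as the placement actor and its Scene world location as the release point.
; End overlap clears the actor reference and zeroes the location.
; The construction script shifts the Box up by its Z extent.
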(event `self.Box.OnComponentBeginOverlap`
  (params (OverlappedComponent :type "PrimitiveComponent Object Reference") (OtherActor :type "Actor Object Reference") (OtherComp :type "PrimitiveComponent Object Reference") (OtherBodyIndex :type Integer) (bFromSweep :type Boolean) (SweepResult :type "HitResult Structure (by ref)"))
  (bind _returnvalue (`self.GetComponentByClass` OtherActor "/Game/InteractiveObjects/Blueprints/Common/BPC_GrabbableComponent.BPC_GrabbableComponent_C"))
  (`/Engine/EditorBlueprintResources/StandardMacros.IsValid` _returnvalue
    (:`Is Valid`
      (set `/Game/InteractiveObjects/Blueprints/Common/BPC_GrabbableComponent.ActorToBePlacedRef` (`self.MyOwner`) _returnvalue)
      (set `/Game/InteractiveObjects/Blueprints/Common/BPC_GrabbableComponent.DesiredReleasePlace` (`SceneComponent.K2_GetComponentLocation` (`self.Scene`)) _returnvalue))))

(event `self.Box.OnComponentEndOverlap`
  (params (OverlappedComponent :type "PrimitiveComponent Object Reference") (OtherActor :type "Actor Object Reference") (OtherComp :type "PrimitiveComponent Object Reference") (OtherBodyIndex :type Integer))
  (bind _returnvalue (`self.GetComponentByClass` OtherActor "/Game/InteractiveObjects/Blueprints/Common/BPC_GrabbableComponent.BPC_GrabbableComponent_C"))
  (`/Engine/EditorBlueprintResources/StandardMacros.IsValid` _returnvalue
    (:`Is Valid`
      (set `/Game/InteractiveObjects/Blueprints/Common/BPC_GrabbableComponent.DesiredReleasePlace` (0.0 0.0 0.0) _returnvalue)
      (set `/Game/InteractiveObjects/Blueprints/Common/BPC_GrabbableComponent.ActorToBePlacedRef` null _returnvalue))))

(fn `UserConstructionScript`
  (bind _box (`self.Box`))
  (`SceneComponent.K2_SetRelativeLocation` _box (+ (`SceneComponent.RelativeLocation` _box) (`KismetMathLibrary.MakeVector` 0.0 0.0 (.z (`BoxComponent.BoxExtent` (`self.Box`))))) false false))