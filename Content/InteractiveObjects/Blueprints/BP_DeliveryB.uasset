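; BP_DeliveryB is an interactive delivery point where buckets of mixed paint are submitted to customers.
; On interact release, it compares the bucket's color intensity against each customer in the player controller's list within a small tolerance.
; A match plays a success sound, removes that customer through the game mode, destroys the bucket and briefly raises a success flag.
; Otherwise it plays a failure sound, records a wrong submission and destroys the bucket.
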(event `self.ReceiveBeginPlay`
  (bind _returnvalue (`GameplayStatics.GetPlayerController` 0))
  (`parent.ReceiveBeginPlay`)
  (cast `/Game/Core/BP_PainterGameMode` (`GameplayStatics.GetGameMode`))
  (`self.EnableInput` _returnvalue)
  (bind _asbp_painter_controller (cast `/Game/Core/BP_PainterController` _returnvalue))
  (set `self.BP_PainterControllerAgain` _asbp_painter_controller))

(event `/Game/Core/BPI_Interact.Release Interact`
  (params (ReleasedInteractiveActor :type "/Game/InteractiveObjects/Blueprints/Common/BP_InteractiveActorBase Object Reference") (`ReleasedActor(Bucket)` :type "Actor Object Reference"))
  (bind _asbp_bucket (cast `/Game/InteractiveObjects/Blueprints/BP_Bucket` `ReleasedActor(Bucket)`))
  (bind _asbp_painter_controller (cast `/Game/Core/BP_PainterController` (`GameplayStatics.GetPlayerController` 0)))
  (if (`KismetArrayLibrary.Array_IsValidIndex` (`/Game/Core/BP_PainterGameMode.CustomerStructure` (`self.PainterGameModeRef`)))
    (for (_array_element _array_index) (`/Game/Core/BP_PainterController.ControllerCustomerList` _asbp_painter_controller)
      (bind _output_get (set `self.ColorDebug` (`.CustumerColorInPercent_10_C7B6C8DC46ED328E696026B443175EA9` (break `/Game/UI/S_CustomerStructure` _array_element))))
      (if (== _output_get (`/Game/InteractiveObjects/Blueprints/BP_Bucket.BucketColorIntensity` _asbp_bucket) :`ErrorTolerance` 0.05)
        (`GameplayStatics.SpawnSound2D` "/Game/Audio/CorrectDelivery.CorrectDelivery" 1.0 1.0 0.0 null)
        (`/Game/Core/BP_PainterGameMode.RemoveSatisfiedCustomer` (`self.PainterGameModeRef`) _array_index)
        (`/Game/InteractiveObjects/Blueprints/BP_Bucket.MyBucketDestroy` _asbp_bucket)
        (`|ExecutionSequence`
          (:`then_0`
            (`/Game/Core/BP_PainterGameMode.UpdateCustomerSubmissions` (cast `/Game/Core/BP_PainterGameMode` (`GameplayStatics.GetGameMode`) :!pure true) true)
            (break))
          (:`then_1`
            (set `self.bSucced` true)
            (`KismetSystemLibrary.Delay` 1.0)
            (set `self.bSucced` false)))))
    (if (not (`self.bSucced`))
      (`GameplayStatics.SpawnSound2D` "/Game/Audio/WrongDelivery.WrongDelivery" 1.0 1.0 0.0 null)
      (`/Game/Core/BP_PainterGameMode.UpdateWrongSubmission` (cast `/Game/Core/BP_PainterGameMode` (`GameplayStatics.GetGameMode`) :!pure true))
      (`/Engine/EditorBlueprintResources/StandardMacros.IsValid` _asbp_bucket
        (:`Is Valid`
          (`KismetSystemLibrary.PrintText` (`|FormatText` "Delivery Complete is trying to kill {Bucket}" _asbp_bucket))
          (`/Game/InteractiveObjects/Blueprints/BP_Bucket.MyBucketDestroy` _asbp_bucket))))))

(fn `UserConstructionScript`
  (`parent.UserConstructionScript`))