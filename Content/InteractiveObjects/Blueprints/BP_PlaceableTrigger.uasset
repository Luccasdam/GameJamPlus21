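; BP_PlaceableTrigger is an interactive placement spot where the painter character can set down a grabbed object.
; On painter interaction with a valid grabbed actor, it detaches the held object and attaches it to its Box, snapping location while keeping world rotation and scale.
; Box overlaps set the desired release place on actors with BPC_GrabbableComponent to the Box's location, resetting it to a zero vector on exit.
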(event `/Game/Core/BPI_Interact.PainterInteract`
  (params (InstigatorPainterChar :type "/Game/PlayerCharacter/BP_PlayerCharacterBase Object Reference") (GrabbedInteractiveActor :type "/Game/InteractiveObjects/Blueprints/BP_InteractiveActorBase Object Reference") (bGrab :type Boolean))
  (bind _grabbedobj (`/Game/PlayerCharacter/BP_PlayerCharacterBase.GrabbedObj` InstigatorPainterChar))
  (`/Engine/EditorBlueprintResources/StandardMacros.IsValid` GrabbedInteractiveActor
    (:`Is Valid`
      (`self.K2_DetachFromActor` _grabbedobj "KeepWorld" "KeepWorld" "KeepWorld")
      (`self.K2_AttachToComponent` _grabbedobj (`self.Box`) "None" "SnapToTarget" "KeepWorld" "KeepWorld" true))))

(event `self.Box.OnComponentBeginOverlap`
  (params (OverlappedComponent :type "PrimitiveComponent Object Reference") (OtherActor :type "Actor Object Reference") (OtherComp :type "PrimitiveComponent Object Reference") (OtherBodyIndex :type Integer) (bFromSweep :type Boolean) (SweepResult :type "HitResult Structure (by ref)"))
  (bind _returnvalue (`self.GetComponentByClass` OtherActor "/Game/InteractiveObjects/Blueprints/BPC_GrabbableComponent.BPC_GrabbableComponent_C"))
  (`/Engine/EditorBlueprintResources/StandardMacros.IsValid` _returnvalue
    (:`Is Valid`
      (set `/Game/InteractiveObjects/Blueprints/BPC_GrabbableComponent.DesiredReleasePlace` (`SceneComponent.K2_GetComponentLocation` (`self.Box`)) _returnvalue))))

(event `self.Box.OnComponentEndOverlap`
  (params (OverlappedComponent :type "PrimitiveComponent Object Reference") (OtherActor :type "Actor Object Reference") (OtherComp :type "PrimitiveComponent Object Reference") (OtherBodyIndex :type Integer))
  (bind _returnvalue (`self.GetComponentByClass` OtherActor "/Game/InteractiveObjects/Blueprints/BPC_GrabbableComponent.BPC_GrabbableComponent_C"))
  (`/Engine/EditorBlueprintResources/StandardMacros.IsValid` _returnvalue
    (:`Is Valid`
      (set `/Game/InteractiveObjects/Blueprints/BPC_GrabbableComponent.DesiredReleasePlace` (0.0 0.0 0.0) _returnvalue))))

(fn `UserConstructionScript`)