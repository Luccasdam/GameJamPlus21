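; BPC_GrabbableComponent is a component that lets its owning actor be grabbed and released by a player.
; On grab, the owner attaches to the player's GrabLocationSceneComponent, snapping position while keeping world rotation and scale.
; On release, it detaches and teleports to DesiredReleasePlace, or, if that is near zero, to the result of a short downward visibility trace, without checking for a hit.
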(event `GetGrabbed`
  (params (InstigatorPlayerBase :type "/Game/PlayerCharacter/BP_PlayerCharacterBase Object Reference"))
  (`Actor.K2_AttachToComponent` (`self.GetOwner`) (`/Game/PlayerCharacter/BP_PlayerCharacterBase.GrabLocationSceneComponent` InstigatorPlayerBase) "None" "SnapToTarget" "KeepWorld" "KeepWorld" true))

(event `GetReleased`
  (bind _returnvalue (`Actor.K2_GetActorLocation` (`self.GetOwner`)))
  (`Actor.K2_DetachFromActor` (`self.GetOwner`) "KeepWorld" "KeepWorld" "KeepWorld")
  (if (!= (`self.DesiredReleasePlace`) (0.0 0.0 0.0) :`ErrorTolerance` 0.1)
    (`Actor.K2_SetActorLocation` (`self.GetOwner`) (`self.DesiredReleasePlace`) false true)
    (else
      (bind _outhit (`KismetSystemLibrary.LineTraceSingle` _returnvalue (- _returnvalue (0.0 0.0 200.0)) "TraceTypeQuery1"))
      (`Actor.K2_SetActorLocation` (`self.GetOwner`) (`.Location` (`GameplayStatics.BreakHitResult` _outhit)) false true))))