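; BP_Bucket is a paint bucket actor that gets filled with color and is respawned through BP_PainterGameMode when destroyed.
; Each refill adds to the accumulated color and liquid count, then swaps the liquid mesh and tints it while levels remain.
; Destruction requests a respawn by bucket index, hides the bucket and disables collision before a delayed destroy.
; An event toggles movement collision with the instigating player; grabbable-owner and reset logic is unconnected.
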(event `self.ReceiveBeginPlay`)

(event `self.IgnorePlayerCollision`
  (params (InstigatorPlayer :type "/Game/Core/PlayerCharacter/BP_PlayerCharacterBase Object Reference") (bIgnorePlayer :type Boolean))
  (`PrimitiveComponent.IgnoreActorWhenMoving` (`self.StaticMesh`) InstigatorPlayer bIgnorePlayer))

(event `self.RefillActor`
  (params (ColorIntensity :type "Vector Structure"))
  (bind _staticmeshliquid (`self.StaticMeshLiquid`))
  (set `self.BucketColorIntensity` (+ ColorIntensity (`self.BucketColorIntensity`)))
  (bind _result (`/Engine/EditorBlueprintResources/StandardMacros.IncrementInt` (`self.BucketLiquidAmount`))
    (:`  `
      (if (<= _result (`KismetArrayLibrary.Array_LastIndex` _staticmeshliquid))
        (`StaticMeshComponent.SetStaticMesh` (`self.StaticMesh1`) (`|GetArrayItem` _staticmeshliquid _result))
        (`MeshComponent.SetVectorParameterValueOnMaterials` (`self.StaticMesh1`) "TintColorIntensity" (`self.BucketColorIntensity`))))))

(event `MyBucketDestroy`
  (`/Game/Core/BP_PainterGameMode.RespawnBucket` (cast `/Game/Core/BP_PainterGameMode` (`GameplayStatics.GetGameMode`) :!pure true) (`self.BucketIndex`))
  (`PrimitiveComponent.SetCollisionEnabled` (`self.StaticMesh`) "NoCollision")
  (`SceneComponent.SetVisibility` (`self.StaticMesh`) false true)
  (`KismetSystemLibrary.Delay` 0.5)
  (`self.K2_DestroyActor`))

(fn `UserConstructionScript`)