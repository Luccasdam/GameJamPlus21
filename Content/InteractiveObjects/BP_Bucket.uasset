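; BP_Bucket is an interactive bucket that a painter character can pick up and put down.
; PainterInteract toggles on the character's Grabbing flag: when it is false, the bucket attaches to GrabSocket and teleports to GrabRelativeLocation.
; When the flag is already true, the bucket clears it and detaches, keeping its world transform.
; Refill only prints a debug message and changes no bucket state.
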(event `self.Refill`
  (`KismetSystemLibrary.PrintString` "Bucked Refilled"))

(event `/Game/Core/BPI_Interact.PainterInteract`
  (params (InstigatorPainterChar :type "/Game/Core/BP_PainterCharacter Object Reference"))
  (if (not (`/Game/Core/BP_PainterCharacter.bGrabbing` InstigatorPainterChar))
    (set `/Game/Core/BP_PainterCharacter.bGrabbing` true InstigatorPainterChar)
    (`self.K2_AttachToActor` InstigatorPainterChar "GrabSocket" "SnapToTarget" "KeepRelative" "KeepRelative" false)
    (`self.K2_SetActorRelativeLocation` (`self.GrabRelativeLocation`) false true)
    (else
      (set `/Game/Core/BP_PainterCharacter.bGrabbing` false InstigatorPainterChar)
      (`self.K2_DetachFromActor` "KeepWorld" "KeepWorld" "KeepWorld"))))

(fn `UserConstructionScript`)