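; Level-building actor that lays out a flat grid of one chosen mesh as instances in an InstancedStaticMesh component.
; The Construction Script sets the mesh behind a DoOnce, prints its bounds and adds the first row along X.
; A second sequence branch adds the remaining rows along Y, using ColummAmount and RowAmount as grid size.
; Spacing comes from unscaled mesh bounds, while each instance takes the actor's scale.
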(fn `UserConstructionScript`
  (`|ExecutionSequence`
    (:`then_0`
      (`/Engine/EditorBlueprintResources/StandardMacros.DoOnce` false
        (:`Completed`
          (bind _output_get (set `self.MeshBounds` (* (`.BoxExtent` (`KismetMathLibrary.BreakBoxSphereBounds` (`StaticMesh.GetBounds` (`self.MeshToInstanciate`)))) 2.0)))
          (`KismetSystemLibrary.PrintString` (`KismetStringLibrary.Conv_VectorToString` _output_get))
          (`StaticMeshComponent.SetStaticMesh` (`self.InstancedStaticMesh`) (`self.MeshToInstanciate`))
          (`InstancedStaticMeshComponent.AddInstance` (`self.InstancedStaticMesh`) (`KismetMathLibrary.MakeTransform` (0.0 0.0 0.0) (struct) (.scale (`self.GetTransform`))))
          (for _index (range 1 (`self.ColummAmount`))
            (`InstancedStaticMeshComponent.AddInstance` (`self.InstancedStaticMesh`) (`KismetMathLibrary.MakeTransform` (`KismetMathLibrary.MakeVector` (* _index (.x (`self.MeshBounds`)))) (struct) (.scale (`self.GetTransform`))))))))
    (:`then_1`
      (for _index_2 (range 1 (`self.RowAmount`))
        (bind _returnvalue (* _index_2 (.y (`self.MeshBounds`))))
        (`InstancedStaticMeshComponent.AddInstance` (`self.InstancedStaticMesh`) (`KismetMathLibrary.MakeTransform` (`KismetMathLibrary.MakeVector` 0.0 _returnvalue) (struct) (.scale (`self.GetTransform`))))
        (for _index_3 (range 1 (`self.ColummAmount`))
          (`InstancedStaticMeshComponent.AddInstance` (`self.InstancedStaticMesh`) (`KismetMathLibrary.MakeTransform` (`KismetMathLibrary.MakeVector` (* _index_3 (.x (`self.MeshBounds`))) _returnvalue) (struct) (.scale (`self.GetTransform`)))))))))