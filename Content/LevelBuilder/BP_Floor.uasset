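; BP_Floor is a level-building actor that tiles a mesh into a rectangular floor grid at construction time.
; The Construction Script measures the mesh's local bounds to space Instanced Static Mesh instances along X and Y using the column and row counts.
; A DoOnce-gated pass lays the origin tile and first line, then nested loops add the remaining rows.
; Each instance takes the actor's rotation and scale, but spacing uses unscaled bounds.
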(fn `UserConstructionScript`
  (bind (_min _max) (`StaticMeshComponent.GetLocalBounds` (`self.InstancedStaticMesh`)))
  (`|ExecutionSequence`
    (:`then_0`
      (`/Engine/EditorBlueprintResources/StandardMacros.DoOnce` false
        (:`Completed`
          (set `self.MeshBounds` (- _max _min))
          (`InstancedStaticMeshComponent.AddInstance` (`self.InstancedStaticMesh`) (`KismetMathLibrary.MakeTransform` (0.0 0.0 0.0) (.rotation (`self.GetTransform`)) (.scale (`self.GetTransform`))))
          (for _index (range 1 (+ (`self.ColummAmount`) 1))
            (`InstancedStaticMeshComponent.AddInstance` (`self.InstancedStaticMesh`) (`KismetMathLibrary.MakeTransform` (`KismetMathLibrary.MakeVector` (* _index (.x (`self.MeshBounds`)))) (.rotation (`self.GetTransform`)) (.scale (`self.GetTransform`))))))))
    (:`then_1`
      (for _index_2 (range 1 (+ (`self.RowAmount`) 1))
        (bind _returnvalue (* _index_2 (.y (`self.MeshBounds`))))
        (`InstancedStaticMeshComponent.AddInstance` (`self.InstancedStaticMesh`) (`KismetMathLibrary.MakeTransform` (`KismetMathLibrary.MakeVector` 0.0 _returnvalue) (.rotation (`self.GetTransform`)) (.scale (`self.GetTransform`))))
        (for _index_3 (range 1 (+ (`self.ColummAmount`) 1))
          (`InstancedStaticMeshComponent.AddInstance` (`self.InstancedStaticMesh`) (`KismetMathLibrary.MakeTransform` (`KismetMathLibrary.MakeVector` (* _index_3 (.x (`self.MeshBounds`))) _returnvalue) (.rotation (`self.GetTransform`)) (.scale (`self.GetTransform`)))))))))